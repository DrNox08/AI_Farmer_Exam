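; BP_Turrett is a turret actor that turns to face a given target, toggles a firing flash, and shows its state by color.
; LookAtTarget smoothly interpolates the actor's yaw toward the target, while Shoot activates or deactivates the Flash component.
; UpdateMaterial swaps the Cylinder material between gray, red and cyan for the Inactive, Active and Alert states.
; Tick is empty, and an idle-rotation snippet is left unconnected.
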(event Custom|Look%20At%20Target
  (params (Actor%20Target :type Actor%20Object%20Reference) (Delta%20Time :type Float%20%28double-precision%29))
  (if (Utilities|IsValid Actor%20Target)
    (bind _output_get (Variables|Default|SetTarger%20Rotation (Math|Interpolation|RInterpTo (Transformation|GetActorRotation) (Math|Rotator|MakeRotator 0.0 0.0 (.yaw (Math|Rotator|FindLookatRotation (Transformation|GetActorLocation) (Transformation|GetActorLocation Actor%20Target)))) Delta%20Time 2e+01)))
    (Transformation|SetActorRotation _output_get)))

(event Custom|Shoot
  (params (Value :type Boolean))
  (bind _flash (Variables|Default|GetFlash))
  (if Value
    (Components|Activation|Activate _flash false)
    (else
      (Components|Activation|Deactivate _flash))))

(event EventTick
  (params (DeltaSeconds :type Float%20%28single-precision%29)))

(fn ConstructionScript)

(fn UpdateMaterial
  (params (State :type E_TurretState%20Enum :default "NewEnumerator0"))
  (switch Utilities|FlowControl|Switch|SwitchonE_TurretState State
    (:NewEnumerator0
      (Rendering|Material|SetMaterial (Variables|Default|GetCylinder) 0 "/Game/Game/Materials/Opaque/M_Gray.M_Gray"))
    (:NewEnumerator1
      (Rendering|Material|SetMaterial (Variables|Default|GetCylinder) 0 "/Game/Game/Materials/Opaque/M_Red.M_Red"))
    (:NewEnumerator2
      (Rendering|Material|SetMaterial (Variables|Default|GetCylinder) 0 "/Game/Game/Materials/Opaque/M_Cyan.M_Cyan"))))