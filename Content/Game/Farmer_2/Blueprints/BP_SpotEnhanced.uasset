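; Farming plot spot that accepts a seed and tracks whether it is free for planting.
; PlantInSpot tells the given seed actor it is planted, fires the OnInitGrowth dispatcher, then marks the spot unavailable.
; The spot starts available on BeginPlay and exposes functions to set and query that flag.
; Growth logic is left to whatever handles the dispatcher.
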(event Custom|Plant%20In%20Spot
  (params (Seed%20Actor :type BP%20Seed%20Enhanced%20Object%20Reference))
  (Default|GetPlanted Seed%20Actor)
  (Default|CallOnInitGrowth self)
  (CallFunction|SetasUnavailable))

(event EventBeginPlay
  (Variables|Default|SetIs%20Available true))

(fn ConstructionScript)

(fn SetasAvailable
  (Variables|Default|SetIs%20Available true))

(fn SetasUnavailable
  (Variables|Default|SetIs%20Available false))

(fn IsSpotAvailable
  (return (Variables|Default|GetIs%20Available)))