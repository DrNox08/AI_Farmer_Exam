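; BP_PlantField is a farm field actor that manages planting spots and a pool of reusable plants.
; Construction records the locations of the Plane's child components; BeginPlay spawns a spot at each and one pooled plant 500 units below the field.
; InitPlantgrowth takes a pooled plant and spawns it at the spot.
; ReturnPlant re-pools it and frees the spot through a location-keyed map, with debug spheres drawn.
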(event Custom|Init%20Plant%20growth
  (params (Spot%20Actor :type BP%20Spot%20Enhanced%20Object%20Reference))
  (bind _output_get (CallFunction|GetPlantfromPool))
  (Default|SpawnPlant _output_get (Transformation|GetActorLocation Spot%20Actor)))

(event EventBeginPlay
  (bind _returnvalue (Transformation|GetActorLocation))
  ;[0.15 0.15 0.15 0.5] SPAWN SPOTS
  (for _array_element (Variables|Default|GetSpotsLocations)
    (bind _returnvalue_2 (Game|SpawnActorfromClass "/Game/Game/Farmer_2/Blueprints/BP_SpotEnhanced.BP_SpotEnhanced_C" (Math|Transform|MakeTransform _array_element "0, 0, 0" "1.000000,1.000000,1.000000") "AlwaysSpawn" "MultiplyWithRoot" 0 0))
    ;[0.15 0.15 0.15 0.5] BIND TO PLANTING EVENT
    (EventDispatchers|BindEventtoOnInitGrowth _returnvalue_2 (EventDispatchers|CreateEvent :!event Custom|Init%20Plant%20growth))
    ;[0.15 0.15 0.15 0.5] CREATE SPOT MAP
    (Utilities|Map|Add (Variables|Default|GetSpot%20Map) _array_element _returnvalue_2)
    ;[0.15 0.15 0.15 0.5] CREATE PLANTS POOL
    (bind _output_get (Variables|Default|SetPool%20Location (Math|Vector|MakeVector (.x _returnvalue) (.y _returnvalue) (- (.z _returnvalue) 5e+02))))
    (bind _returnvalue_3 (Game|SpawnActorfromClass "/Game/Game/Farmer_2/Blueprints/BP_PlantEnhanced.BP_PlantEnhanced_C" (Math|Transform|MakeTransform _output_get "0, 0, 0" "1.000000,1.000000,1.000000") "Undefined" "MultiplyWithRoot" 0 0))
    (Utilities|Array|AddUnique (Variables|Default|GetPlant%20Pool) _returnvalue_3)
    ;[0.15 0.15 0.15 0.5] BIND TO PLANT EVENTS
    (EventDispatchers|BindEventtoOnPlantDeposited _returnvalue_3 (EventDispatchers|CreateEvent :!event ReturnPlant))
    (bind _keypin (Utilities|Map|ForEachLoop(Map) (Variables|Default|GetSpot%20Map))
      (:then
        (Rendering|Debug|DrawDebugSphere _keypin 1e+02 12 "(R=0.000000,G=0.078063,B=1.000000,A=1.000000)" 1e+01 1.0)))))

(fn ConstructionScript
  (for _array_element (Components|GetChildrenComponents (Variables|Default|GetPlane) false)
    (Utilities|Array|Add (Variables|Default|GetSpotsLocations) (Transformation|GetWorldLocation _array_element))
    (Rendering|Debug|DrawDebugSphere (Transformation|GetWorldLocation _array_element) 1e+01 12 "(R=1.000000,G=0.000552,B=0.000000,A=1.000000)" 1e+01 1.0)))

(fn GetPlantfromPool
  (bind _plant_pool (Variables|Default|GetPlant%20Pool))
  (bind _output_get (LocalVariables|SetPlant%20Actor (Utilities|Array|Get(acopy) _plant_pool)))
  (Utilities|Array|RemoveItem _plant_pool _output_get)
  (return _output_get))

(fn ReturnPlant
  (params (Plant%20Actor :type BP%20Plant%20Enhanced%20Object%20Reference) (Spot%20Location :type Vector))
  (Transformation|SetActorLocation Plant%20Actor (Variables|Default|GetPool%20Location) false false)
  (Transformation|SetActorRotation Plant%20Actor)
  (Utilities|Array|Add (Variables|Default|GetPlant%20Pool) Plant%20Actor)
  (CallFunction|EnableRelativeSpot Spot%20Location))

(fn EnableRelativeSpot
  (params (Spot%20Location :type Vector))
  (bind _spot_map (Variables|Default|GetSpot%20Map))
  (bind (_value _returnvalue) (Utilities|Map|Find _spot_map Spot%20Location))
  (if _returnvalue
    (Default|SetasAvailable _value)
    (Rendering|Debug|DrawDebugSphere Spot%20Location 1e+01 12 "(R=0.000000,G=0.028139,B=1.000000,A=1.000000)" 5.0 1.0)
    (else
      (Development|PrintString "SPOT NOT FOUND" true true "(R=0.000000,G=0.660000,B=1.000000,A=1.000000)" 1e+01))))