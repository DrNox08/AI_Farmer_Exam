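; BP_PlantEnhanced is a farm plant actor that grows for a set time and then becomes ready.
; SpawnPlant stores and moves it to the given location, applies the growing material to its cone mesh and starts a timer.
; When the timer fires, SetPlantReady swaps to the ready material and sets IsReady, which IsPlantReady exposes.
; NotifyPlantDeposited broadcasts the plant and its spot location through OnPlantDeposited, then clears the ready state.
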(event Custom|Spawn%20Plant
  (params (Spawn%20Location :type Vector))
  (bind _output_get (Variables|Default|SetSpawn%20Location Spawn%20Location))
  (Transformation|SetActorLocation _output_get false false)
  (Rendering|Material|SetMaterial (Variables|Default|GetCone) 0 (Variables|Default|GetM_Growing))
  (Utilities|Time|SetTimerbyEvent (delegate Custom|Set%20Plant%20Ready) (Variables|Default|GetGrowing%20Time)))

(event Custom|Set%20Plant%20Ready
  (Rendering|Material|SetMaterial (Variables|Default|GetCone) 0 (Variables|Default|GetM_Ready))
  (CallFunction|SetasReady))

(event EventBeginPlay)

(fn ConstructionScript)

(fn SetasReady
  (Variables|Default|SetIs%20Ready true))

(fn ResetState
  (Variables|Default|SetIs%20Ready false))

(fn NotifyPlantDeposited
  (Default|CallOnPlantDeposited self (Variables|Default|GetSpawn%20Location))
  (CallFunction|ResetState))

(fn IsPlantReady
  (return (Variables|Default|GetIs%20Ready)))