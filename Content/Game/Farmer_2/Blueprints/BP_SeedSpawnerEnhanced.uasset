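; Seed spawner actor that keeps a pre-spawned pool of BP_SeedEnhanced actors and makes them available in the world one at a time.
; BeginPlay fills the pool at a holding location, binds each seed's picked and planted events, and starts a looping timer.
; The timer teleports a pooled seed to the spawner's location whenever the CanSpawn flag allows.
; Helper functions re-enable spawning or return seeds to the pool for reuse.
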(event Custom|Start%20Spawning
  ;[0.15 0.15 0.15 0.5] EVERY X SECONDS, TAKES A SEED FROM POOL AND SET ITS LOCATION INSIDE THE NAVMESH BOUND VOLUME
  (Utilities|Time|SetTimerbyEvent (delegate Custom|Spawn%20Seed) 3.0 true))

(event Custom|Spawn%20Seed
  ;[0.15 0.15 0.15 0.5] EVERY X SECONDS, TAKES A SEED FROM POOL AND SET ITS LOCATION INSIDE THE NAVMESH BOUND VOLUME
  (Variables|Default|GetCan%20Spawn
    (:then
      (Variables|Default|SetCan%20Spawn false)
      (bind _seed_actor (CallFunction|GetSeedfromPool))
      (Transformation|SetActorLocation _seed_actor (Transformation|GetActorLocation) false true))
    (:else)))

(event EventBeginPlay
  (for _index (range 0 20)
    (bind _returnvalue (Game|SpawnActorfromClass "/Game/Game/Farmer_2/Blueprints/BP_SeedEnhanced.BP_SeedEnhanced_C" (Math|Transform|MakeTransform (Transformation|GetWorldLocation (Variables|Default|GetPool%20Location)) "0, 0, 0" "1.000000,1.000000,1.000000") "Undefined" "MultiplyWithRoot" 0 0))
    ;[0.15 0.15 0.15 0.5] ADD SEED TO THE POOL AND BIND TO ITS EVENTS
    (Utilities|Array|Add (Variables|Default|GetSeed%20Pool) _returnvalue)
    (EventDispatchers|BindEventtoOnSeedPicked _returnvalue (EventDispatchers|CreateEvent :!event SetCanSpawn))
    (EventDispatchers|BindEventtoOnSeedPlanted _returnvalue (EventDispatchers|CreateEvent :!event ReturnSeed))
    ;[0.15 0.15 0.15 0.5] START SPAWNING IMMEDIATELY
    (Variables|Default|SetCan%20Spawn true)
    (CallFunction|StartSpawning)))

(fn ConstructionScript)

(fn GetSeedfromPool
  (bind _seed_pool (Variables|Default|GetSeed%20Pool))
  (bind _output_get (LocalVariables|SetNewLocalVar (Utilities|Array|Get(acopy) _seed_pool)))
  (Utilities|Array|RemoveItem _seed_pool _output_get)
  (return _output_get))

(fn ReturnSeed
  (params (Seed%20Actor :type BP%20Seed%20Enhanced%20Object%20Reference))
  ;[0.15 0.15 0.15 0.5] SET LOCATION TO POOL LOCATION
  (Transformation|SetActorLocation Seed%20Actor (Transformation|GetWorldLocation (Variables|Default|GetPool%20Location)) false true)
  ;[0.15 0.15 0.15 0.5] ADD BACK TO POOL ARRAY
  (Utilities|Array|Add (Variables|Default|GetSeed%20Pool) Seed%20Actor))

(fn SetCanSpawn
  (params (Seed%20Actor :type BP%20Seed%20Enhanced%20Object%20Reference))
  ;[0.15 0.15 0.15 0.5] REMOVE SEED FORM ARRAY AND SET CAN SPAWN TO TRUE
  (Utilities|Array|RemoveItem (Variables|Default|GetSeed%20Pool) Seed%20Actor)
  (Variables|Default|SetCan%20Spawn true))