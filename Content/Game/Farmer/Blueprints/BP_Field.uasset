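; BP_Field is a farm field actor that manages plants at fixed planting spots.
; Its construction script records the world locations of the Plane component's children as spots.
; BeginPlay spawns a hidden, pre-created plant and a BP_Spot with debug sphere at each, binds plant-picked events, and maps locations to plants.
; StartGrowth starts a timer for mapped spots, with no visible link to EnablePlant, which unhides plants.
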(event EventBeginPlay
  (Utilities|FlowControl|Sequence
    (:then_0
      (for _array_element (Variables|Default|GetSpots)
        (bind _returnvalue (Game|SpawnActorfromClass "/Game/Game/Farmer/Blueprints/BP_Plant.BP_Plant_C" (Math|Transform|MakeTransform _array_element "0, 0, 0" "1.000000,1.000000,1.000000") "AlwaysSpawn" "MultiplyWithRoot" 0 0))
        (Utilities|Array|AddUnique (Variables|Default|GetPlants) _returnvalue)
        (CallFunction|DisablePlant _returnvalue)
        (EventDispatchers|BindEventtoOnPlantPicked _returnvalue (EventDispatchers|CreateEvent :!event DisablePlant))))
    (:then_1
      (for _array_element_2 (Variables|Default|GetSpots)
        (Game|SpawnActorfromClass "/Game/Game/Farmer/Blueprints/BP_Spot.BP_Spot_C" (Math|Transform|MakeTransform _array_element_2 "0, 0, 0" "1.000000,1.000000,1.000000") "Undefined" "MultiplyWithRoot" 0 0)
        (Rendering|Debug|DrawDebugSphere _array_element_2 5e+01 12 "(R=1.000000,G=0.139205,B=0.038736,A=1.000000)" 999.0 1.0)))
    (:then_2
      (for (_array_element_3 _array_index) (Variables|Default|GetSpots)
        (Utilities|Map|Add (Variables|Default|GetPlantMap) _array_element_3 (Utilities|Array|Get(acopy) (Variables|Default|GetPlants) _array_index))))))

(fn ConstructionScript
  (for _array_element (Components|GetChildrenComponents (Variables|Default|GetPlane) false)
    (Utilities|Array|AddUnique (Variables|Default|GetSpots) (Transformation|GetWorldLocation _array_element))))

(fn DisablePlant
  (params (Plant%20Actor :type BP%20Plant%20Object%20Reference))
  (if (Utilities|Array|ContainsItem (Variables|Default|GetPlants) Plant%20Actor)
    (Rendering|SetActorHiddenInGame Plant%20Actor true)))

(fn StartGrowth
  (params (Spot%20Position :type Vector))
  (if (.ReturnValue (Utilities|Map|Find (Variables|Default|GetPlantMap) Spot%20Position))
    (Utilities|Time|SetTimerbyEvent 0 (Variables|Default|GetGrowthTime))))

(fn EnablePlant
  (params (Plant%20Actor :type BP%20Plant%20Object%20Reference))
  (Rendering|SetActorHiddenInGame Plant%20Actor false))