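; BP_SeedSpawner is an actor that spawns farming seeds at its own location using an object pool.
; On BeginPlay it pre-spawns BP_Seed actors at the Pool component's position and starts a looping timer for spawning.
; A CanSpawn flag holds back the next seed until the current one reports being picked.
; Seeds are taken from the pool array, with a Repool function to return them to storage.
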(event Custom|SpawnSeed
  (Variables|Default|GetCanSpawn
    (:then
      (Variables|Default|SetCanSpawn false)
      (bind _array_element (CallFunction|GetSeedfromPool))
      (Transformation|SetActorLocation _array_element (.location (Transformation|GetActorTransform)) false false)
      (EventDispatchers|BindEventtoOnSeedPicked _array_element (delegate Custom|Set%20Can%20Spawn))
      (EventDispatchers|BindEventtoOnSeedEndLife _array_element (EventDispatchers|CreateEvent :!event Repool)))
    (:else
      (Development|PrintString "CAN NOT SPAWN" true true "(R=1.000000,G=0.000000,B=0.021475,A=1.000000)"))))

(event Custom|Set%20Can%20Spawn
  (Variables|Default|SetCanSpawn true)
  (Development|PrintString "SEED PICKED"))

(event EventBeginPlay
  (CallFunction|CratePool)
  (CallFunction|StartSpawnTimer)
  (Rendering|Debug|DrawDebugSphere (Transformation|GetWorldLocation (Variables|Default|GetPool%20)) 1e+02 12 "(R=1.000000,G=1.000000,B=1.000000,A=1.000000)" 999.0 1.0))

(fn ConstructionScript)

(fn CratePool
  (for _index (range 0 50)
    (bind _returnvalue (Game|SpawnActorfromClass "/Game/Game/Farmer/Blueprints/BP_Seed.BP_Seed_C" (Math|Transform|MakeTransform (Transformation|GetWorldLocation (Variables|Default|GetPool%20)) "0, 0, 0" "1.000000,1.000000,1.000000") "Undefined" "MultiplyWithRoot" 0 0))
    (Utilities|Array|AddUnique (Variables|Default|GetSeed%20Pool) _returnvalue)))

(fn Repool
  (params (Seed :type BP%20Seed%20Object%20Reference))
  (Utilities|Array|AddUnique (Variables|Default|GetSeed%20Pool) Seed)
  (Transformation|SetActorLocation Seed (Transformation|GetWorldLocation (Variables|Default|GetPool%20)) false true))

(fn GetSeedfromPool
  (bind _seed_pool (Variables|Default|GetSeed%20Pool))
  (bind _output (Utilities|Array|Get(acopy) _seed_pool))
  (bind _output_get (LocalVariables|SetSeed%20Actor _output))
  (Utilities|Array|RemoveItem _seed_pool _output)
  (return _output_get))

(fn StartSpawnTimer
  (Variables|Default|SetCanSpawn true)
  (bind _returnvalue (Utilities|Time|SetTimerbyEvent (EventDispatchers|CreateEvent :!event Custom|SpawnSeed) 1.0 true))
  (Variables|Default|SetTimerHandle _returnvalue))