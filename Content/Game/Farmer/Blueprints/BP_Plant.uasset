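; BP_Plant is a farm plant that appears after a growth timer and can be picked up.
; Spawn and despawn move the same actor between stored enabled and disabled positions rather than creating or destroying it.
; StartGrowth sets the timer that triggers Spawn, which teleports the plant to its enabled position.
; Picking attaches it to the given component's HandSocket and, on success, fires the OnPlantPicked dispatcher.
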(event Custom|Start%20Growth
  (params (Growth%20Time :type Float%20%28double-precision%29))
  (Utilities|Time|SetTimerbyEvent (delegate Custom|Spawn) Growth%20Time))

(event Custom|Spawn
  (Transformation|SetActorLocation (Variables|Default|GetEnabled%20Position) false true))

(event Custom|Despawn
  (Transformation|SetActorLocation (Variables|Default|GetDisabled%20Position) false false))

(fn ConstructionScript)

(fn SetDisablePosition
  (params (NewParam :type Vector))
  (Variables|Default|SetDisabled%20Position NewParam))

(fn SetEnablePosition
  (Variables|Default|SetEnabled%20Position (Transformation|GetActorLocation)))

(fn GetPicked
  (params (Scene%20Component :type Scene%20Component%20Object%20Reference))
  (bind _returnvalue (Transformation|AttachComponentToComponent Scene%20Component "HandSocket" "SnapToTarget" "SnapToTarget" "KeepRelative" true))
  (if _returnvalue
    (Default|CallOnPlantPicked self)
    (return _returnvalue)))